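; Tunnel VFX actor that spawns a cube-tunnel Niagara system when something overlaps its Box, through a DoOnce that is never reset.
; It passes the system a box size and a fixed-length line from EffectBeginPoint along TunnelDirection.
; Tick feeds it the overlapping actor's position, and end overlap deactivates it.
; BeginPlay disables actor collision, and nothing here re-enables it.
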(event OnComponentBeginOverlap(Box)
  (params (OverlappedComponent :type Primitive%20Component%20Object%20Reference) (OtherActor :type Actor%20Object%20Reference) (OtherComp :type Primitive%20Component%20Object%20Reference) (OtherBodyIndex :type Integer) (bFromSweep :type Boolean) (SweepResult :type Hit%20Result%20Structure%20%28by%20ref%29))
  (bind _effectbeginpoint (Variables|Default|GetEffectBeginPoint))
  (bind _returnvalue (Transformation|GetWorldLocation _effectbeginpoint))
  (Utilities|FlowControl|DoOnce false
    (:Completed
      (if (Utilities|IsValid OtherActor)
        (bind _returnvalue_2 (Niagara|SpawnSystematLocation "/Game/NEffect/Tunnel/NS_Cube_Tunnel_01.NS_Cube_Tunnel_01" (Transformation|GetWorldLocation (Variables|Default|GetBox))))
        (if (Utilities|IsValid _returnvalue_2)
          (bind _output_get (Variables|Default|SetNiagara_Scene_Component _returnvalue_2))
          (Niagara|SetNiagaraVariable(Vector3) _output_get "Line Start" _returnvalue)
          (Niagara|SetNiagaraVariable(Vector3) (Variables|Default|GetNiagara_Scene_Component) "Line End" (+ _returnvalue (* (Variables|Default|GetTunnelDirection) 3.5e+03)))
          (Niagara|SetNiagaraVariable(Vector3) (Variables|Default|GetNiagara_Scene_Component) "Box Size" (* (Variables|/Script/Engine.BoxComponent|GetBoxExtent (Variables|Default|GetBox)) 2.0)))))))

(event OnComponentEndOverlap(Box)
  (params (OverlappedComponent :type Primitive%20Component%20Object%20Reference) (OtherActor :type Actor%20Object%20Reference) (OtherComp :type Primitive%20Component%20Object%20Reference) (OtherBodyIndex :type Integer))
  (if (Utilities|IsValid (Variables|Default|GetNiagara_Scene_Component))
    (Components|Activation|Deactivate (Variables|Default|GetNiagara_Scene_Component))
    (Utilities|FlowControl|Delay 0.5)))

(event EventBeginPlay
  (Collision|SetActorEnableCollision false))

(event Collision|EventActorBeginOverlap
  (params (OtherActor :type Actor%20Object%20Reference)))

(event EventTick
  (params (DeltaSeconds :type Float%20%28single-precision%29))
  (bind _niagara_scene_component (Variables|Default|GetNiagara_Scene_Component))
  (if (Utilities|IsValid _niagara_scene_component)
    (Niagara|SetNiagaraVariable(Vector3) _niagara_scene_component "Player_Position_Update" (Transformation|GetActorLocation (stale OnComponentBeginOverlap(Box) OtherActor)))))

(fn ConstructionScript)